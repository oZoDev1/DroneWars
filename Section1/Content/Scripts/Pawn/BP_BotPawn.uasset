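; Player-controlled flying bot pawn that shoots blaster beams from two rifles and quits the game when its health runs out.
; On BeginPlay it adds the bot input context and HUD; movement follows control rotation through FloatingPawnMovement, and the mesh matches that rotation each tick.
; Firing alternates rifle sockets via FlipFlop, using a camera trace to aim each spawned beam at the view target, with burst effect and sound.
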(event Input|EnhancedActionEvents|EnhancedInputActionIA_Fire
  (params (ActionValue :type Boolean) (ElapsedSeconds :type Float%20%28double-precision%29) (TriggeredSeconds :type Float%20%28double-precision%29) (InputAction :type Input%20Action%20Object%20Reference :default "/Game/Scripts/Pawn/Input/Actions/IA_Fire.IA_Fire"))
  (bind _isa (Utilities|FlowControl|FlipFlop)
    (:A
      _)
    (:B
      _))
  (CallFunction|FireRifle _isa))

(event Input|EnhancedActionEvents|EnhancedInputActionIA_Look
  (params (ActionValue :type Vector%202D%20Structure) (ElapsedSeconds :type Float%20%28double-precision%29) (TriggeredSeconds :type Float%20%28double-precision%29) (InputAction :type Input%20Action%20Object%20Reference :default "/Game/Scripts/Pawn/Input/Actions/IA_Look.IA_Look"))
  (bind (_x _y) (Math|Vector2D|BreakVector2D ActionValue))
  (Pawn|Input|AddControllerYawInput _x)
  (Pawn|Input|AddControllerPitchInput _y))

(event Input|EnhancedActionEvents|EnhancedInputActionIA_Move
  (params (ActionValue :type Vector%202D%20Structure) (ElapsedSeconds :type Float%20%28double-precision%29) (TriggeredSeconds :type Float%20%28double-precision%29) (InputAction :type Input%20Action%20Object%20Reference :default "/Game/Scripts/Pawn/Input/Actions/IA_Move.IA_Move"))
  (bind (_x _y) (Math|Vector2D|BreakVector2D ActionValue))
  (bind _returnvalue (Pawn|GetControlRotation :!class /Script/Engine.Pawn))
  (bind _floatingpawnmovement (Variables|Default|GetFloatingPawnMovement))
  (Class|PawnMovementComponent|AddInputVector _floatingpawnmovement (* _x (Math|Vector|GetRightVector _returnvalue)) false)
  (Class|PawnMovementComponent|AddInputVector _floatingpawnmovement (* _y (Math|Vector|GetForwardVector _returnvalue)) false))

(event EventBeginPlay
  ;[10 0 0 1 22] Input
  (bind _asplayer_controller (Utilities|Casting|CastToPlayerController (Pawn|GetController)))
  (Input|AddMappingContext (PlayerController|LocalPlayerSubsystems|GetEnhancedInputLocalPlayerSubsystem _asplayer_controller) "/Game/Scripts/Pawn/Input/IMC_Bot.IMC_Bot" 0 "(bIgnoreAllPressedKeysUntilRelease=True,bForceImmediately=False,bNotifyUserSettings=False)")
  (bind _returnvalue (UserInterface|CreateWidget "/Game/Scripts/Widgets/WB_OverlayHUD.WB_OverlayHUD_C"))
  (UserInterface|Viewport|AddtoViewport _returnvalue 0))

(event EventGetHurt
  (params (Damage :type Float%20%28double-precision%29))
  (bind _output_get (Variables|Default|SetHealth (- (Variables|Default|GetHealth) Damage)))
  (Development|PrintString (Utilities|String|ToString(Float) _output_get))
  (if (<= (Variables|Default|GetHealth) 0.0)
    (Actor|DestroyActor)
    (Game|QuitGame 0 "Quit" false)))

(event EventTick
  (params (DeltaSeconds :type Float%20%28single-precision%29))
  (Transformation|SetWorldRotation (Variables|Default|GetBotMesh) (Pawn|GetControlRotation :!class /Script/Engine.Pawn) false false))

(fn ConstructionScript)

(fn FireRifle
  (params (isLeftRifle :type Boolean))
  (bind _botmesh (Variables|Default|GetBotMesh))
  (bind _camera (Variables|Default|GetCamera))
  (bind _tracedistance (Variables|Default|GetTraceDistance))
  (bind _returnvalue (Math|Vector|GetForwardVector _camera))
  (bind _returnvalue_2 (Transformation|GetWorldLocation _camera))
  (bind _returnvalue_3 (* _returnvalue _tracedistance))
  (bind _returnvalue_4 (+ _returnvalue_2 _returnvalue_3))
  (LocalVariables|SetTraceEnd _returnvalue_4)
  (bind _outhit (Collision|LineTraceByChannel _returnvalue_2 _returnvalue_4 "TraceTypeQuery1" false 0 "None"))
  (LocalVariables|SetTraceEnd (select (.bBlockingHit (Collision|BreakHitResult _outhit)) (.ImpactPoint (Collision|BreakHitResult _outhit)) (LocalVariables|GetTraceEnd)))
  (if isLeftRifle
    (Variables|Default|SetSocketName "RifleL")
    (else
      (Variables|Default|SetSocketName "RifleR")))
  (Game|SpawnActorfromClass "/Game/Scripts/BlasterBeam/BP_BlasterBeam.BP_BlasterBeam_C" (Math|Transform|MakeTransform (Transformation|GetSocketLocation _botmesh (Variables|Default|GetSocketName)) (Math|Rotator|FindLookatRotation (Transformation|GetSocketLocation _botmesh (Variables|Default|GetSocketName)) (LocalVariables|GetTraceEnd)) "1.000000,1.000000,1.000000") "Undefined" "MultiplyWithRoot" 0 0)
  (Niagara|SpawnSystematLocation "/Game/Scripts/FX/NS_BeamBurst.NS_BeamBurst" (Transformation|GetSocketLocation _botmesh (Variables|Default|GetSocketName)) (Transformation|GetSocketRotation _botmesh (Variables|Default|GetSocketName)))
  (Audio|PlaySoundatLocation "/Game/Models/Sounds/sfx_EnergyRifle.sfx_EnergyRifle" (Transformation|GetSocketLocation _botmesh (Variables|Default|GetSocketName)) "0, 0, 0" 1.0 1.0 0.0 0 0 0 0))