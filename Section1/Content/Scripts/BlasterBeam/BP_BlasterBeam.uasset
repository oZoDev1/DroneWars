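; BP_BlasterBeam is a blaster projectile actor that damages what it hits.
; On begin play it binds to the hit event of its BeamMesh component.
; On impact it spawns a Niagara burst at the impact point aligned to the surface normal, destroys itself, and sends a fixed damage amount through BPI_Damageable if the hit actor implements that interface.
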(event Custom|OnComponentHit_Event
  (params (HitComponent :type Primitive%20Component%20Object%20Reference) (OtherActor :type Actor%20Object%20Reference) (OtherComp :type Primitive%20Component%20Object%20Reference) (NormalImpulse :type Vector) (Hit :type Hit%20Result%20Structure%20%28by%20ref%29))
  (bind (_bblockinghit _binitialoverlap _time _distance _location _impactpoint _normal) (Collision|BreakHitResult Hit))
  (Variables|Default|SetHitActor OtherActor)
  (Niagara|SpawnSystematLocation "/Game/Scripts/FX/NS_BeamBurst.NS_BeamBurst" _impactpoint (Math|Rotator|MakeRotfromX _normal))
  (Actor|DestroyActor)
  (if (Utilities|DoesObjectImplementInterface (Variables|Default|GetHitActor) "/Game/Scripts/Interfaces/BPI_Damageable.BPI_Damageable_C")
    (Class|BPIDamageable|GetHurt(Message) (Variables|Default|GetHitActor) 2e+01)))

(event EventBeginPlay
  (Collision|AssignOnComponentHit (Variables|Default|GetBeamMesh) (delegate Custom|OnComponentHit_Event)))

(fn ConstructionScript)